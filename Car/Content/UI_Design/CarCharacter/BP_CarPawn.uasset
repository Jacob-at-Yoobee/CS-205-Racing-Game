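; Car pawn Blueprint whose only active graph logic is a pause menu toggle on the IA_PauseGame Enhanced Input action.
; Opening creates a new Resume_UI widget, shows the cursor, switches to game-and-UI input and pauses the game.
; Closing removes the widget, unpauses, restores game-only input and hides the cursor, with a boolean tracking the state.
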(event Input|EnhancedActionEvents|EnhancedInputActionIA_PauseGame
  (params (ActionValue :type Boolean) (ElapsedSeconds :type Float%20%28double-precision%29) (TriggeredSeconds :type Float%20%28double-precision%29) (InputAction :type Input%20Action%20Object%20Reference :default "/Game/UI_Design/Actions/IA_PauseGame.IA_PauseGame"))
  (:Started
    (if (not (Variables|Default|GetispausedMenuOpen))
      (Variables|Default|SetispausedMenuOpen true)
      (bind _returnvalue (UserInterface|CreateWidget "/Game/UI_Design/WidgetScreen/Resume_UI.Resume_UI_C"))
      (bind _output_get (Variables|Default|SetPauseMenuWidget _returnvalue))
      (UserInterface|Viewport|AddtoViewport _output_get 0)
      (Input|SetInputModeGameandUI 0 (Variables|Default|GetPauseMenuWidget) "DoNotLock" true false)
      (Variables|/Script/Engine.PlayerController|SetbShowMouseCursor (Game|GetPlayerController 0) true)
      (Game|SetGamePaused true)
      (else
        (Variables|Default|SetispausedMenuOpen false)
        (Widget|RemovefromParent (Variables|Default|GetPauseMenuWidget))
        (Game|SetGamePaused false)
        (Input|SetInputModeGameOnly 0 false)
        (Variables|/Script/Engine.PlayerController|SetbShowMouseCursor (Game|GetPlayerController 0) false)))))

(event EventBeginPlay)

(event Collision|EventActorBeginOverlap
  (params (OtherActor :type Actor%20Object%20Reference)))

(event EventTick
  (params (DeltaSeconds :type Float%20%28single-precision%29)))

(fn ConstructionScript)