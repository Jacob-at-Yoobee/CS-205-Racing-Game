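; Configurable street light prop for city tracks, with optional traffic light, pedestrian crossing signal, transformer box, two signs and two rect lights.
; All logic runs in the Construction Script, driven by variables; the event graph is empty.
; LightId selects red, yellow or green, while CrossingId picks the crossing mesh and layout, with paired walk/stop signals showing opposite states.
; Toggles, mesh arrays and transform offsets configure attachments, and lamp material slots are set alongside the rect lights.
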(event EventBeginPlay)

(event Collision|EventActorBeginOverlap
  (params (OtherActor :type Actor%20Object%20Reference)))

(event EventTick
  (params (DeltaSeconds :type Float%20%28single-precision%29)))

(fn ConstructionScript
  (bind _light1__on_off_ (Variables|Default|Getlight1%20%28on/off%29))
  (bind _transformator (Variables|Default|Gettransformator))
  (bind _light2__on_off_ (Variables|Default|Getlight2%20%28on/off%29))
  (bind _crossing_light (Variables|Default|Getcrossing_light))
  (bind _crossing_id (Variables|Default|Getcrossing_id))
  (bind _crossing_light_stop_l (Variables|Default|Getcrossing_light_stop_l))
  (bind _sign_a (Variables|Default|Getsign_a))
  (bind _sign_b (Variables|Default|Getsign_b))
  (bind _street_light (Variables|Default|Getstreet_light))
  (bind _light_id (Variables|Default|Getlight_id))
  (bind _street_light_2 (Variables|Default|Getstreet_light))
  (bind _crossing_light_stop_r (Variables|Default|Getcrossing_light_stop_r))
  (bind _crossing_light_stop_r_2 (Variables|Default|Getcrossing_light_stop_r))
  (bind _crossing_light__on_off_ (Variables|Default|Getcrossing_light%20%28on/off%29))
  (Rendering|SetVisibility (Variables|Default|Gettraffic_light) (Variables|Default|Gettraffic_light%20%28on/off%29) true)
  (if (== _light_id 0)
    (Rendering|SetVisibility (Variables|Default|Getred) true true)
    (Rendering|SetVisibility (Variables|Default|Getgreen) false true)
    (elif (== _light_id 1)
      (Rendering|SetVisibility (Variables|Default|Getyellow) true true)
      (Rendering|SetVisibility (Variables|Default|Getred) false true)
      (else
        (Rendering|SetVisibility (Variables|Default|Getgreen) true true)
        (Rendering|SetVisibility (Variables|Default|Getred) false true))))
  ;[0.9792 1 1] Crossing light
  (Rendering|SetVisibility _crossing_light _crossing_light__on_off_ true)
  (if _crossing_light__on_off_
    (Components|StaticMesh|SetStaticMesh _crossing_light (Utilities|Array|Get(acopy) (Variables|Default|Getcrossing_meshes) _crossing_id))
    (if (== _crossing_id 0)
      (Class|SceneComponent|AddLocalTransform _crossing_light (Variables|Default|Getcrossing_transform) false false :!label _label)
      (Rendering|SetVisibility (Variables|Default|Getcrossing_light_walk_l) (Variables|Default|Getwalk/stop) true)
      (if (Variables|Default|Getwalk/stop)
        (Variables|Default|Setwalk%20r false)
        (Rendering|SetVisibility _crossing_light_stop_l false true)
        (else
          (Variables|Default|Setwalk%20r true)
          (Rendering|SetVisibility _crossing_light_stop_l true true)))
      (Rendering|SetVisibility (Variables|Default|Getcrossing_light_walk_r) (Variables|Default|Getwalk%20r) true)
      (if (Variables|Default|Getwalk%20r)
        (Variables|Default|Setwalk/stop false)
        (Rendering|SetVisibility _crossing_light_stop_r false true)
        (else
          (Variables|Default|Setwalk/stop true)
          (Rendering|SetVisibility _crossing_light_stop_r true true)))
      (elif (< _crossing_id 2)
        (Class|SceneComponent|AddLocalTransform (Variables|Default|Getligh_root_l) (Variables|Default|Getlight_transform_l) false false)
        (Class|SceneComponent|AddLocalTransform (Variables|Default|Getligh_root_r) (Variables|Default|Getlight_transform_r) false false)
        (goto _label)
        (else
          (if (== _crossing_id 2)
            (Class|SceneComponent|AddLocalTransform (Variables|Default|Getligh_root_r) (Variables|Default|Getlight_transform_l_a) false false)
            (else
              (Class|SceneComponent|AddLocalTransform (Variables|Default|Getligh_root_r) (Variables|Default|Getlight_transform_r_a) false false)))
          (Rendering|SetVisibility (Variables|Default|Getcrossing_light_walk_l) false true)
          (Class|SceneComponent|AddLocalTransform _crossing_light (Variables|Default|Getcrossing_transform) false false)
          (Rendering|SetVisibility (Variables|Default|Getcrossing_light_walk_r) (Variables|Default|Getwalk/stop) true)
          (if (Variables|Default|Getwalk/stop)
            (Rendering|SetVisibility _crossing_light_stop_r_2 false true)
            (else
              (Rendering|SetVisibility _crossing_light_stop_r_2 true true))))))
    (else
      (Rendering|SetVisibility (Variables|Default|Getligh_root_l) false true)))
  (Rendering|SetVisibility _transformator (Variables|Default|Gettransformator%20%28on/off%29) false)
  (Class|SceneComponent|AddLocalTransform _transformator (Variables|Default|Gettransformator_transform) false false)
  ;[1 1 1] sign selector
  (Components|StaticMesh|SetStaticMesh _sign_a (Utilities|Array|Get(acopy) (Variables|Default|Getsign_a_meshes) (Variables|Default|Getsign_a_id)))
  (Rendering|SetVisibility _sign_a (Variables|Default|Getsign%20a%20%28on/off%29) false)
  (Class|SceneComponent|AddLocalTransform _sign_a (Variables|Default|Getsign_a_transform) false false)
  (Components|StaticMesh|SetStaticMesh _sign_b (Utilities|Array|Get(acopy) (Variables|Default|Getsign_b_meshes) (Variables|Default|Getsign_b_id)))
  (Rendering|SetVisibility _sign_b (Variables|Default|Getsign_b%20%28on/off%29) false)
  (Class|SceneComponent|AddLocalTransform _sign_b (Variables|Default|Getsign_b_transform) false false)
  (Rendering|SetVisibility (Variables|Default|GetRectLight1) _light1__on_off_ false)
  (if _light1__on_off_
    (Rendering|Material|SetMaterial _street_light_2 1 0)
    (else
      (Rendering|Material|SetMaterial _street_light_2 1 0)))
  (Rendering|SetVisibility (Variables|Default|GetRectLight2) _light2__on_off_ false)
  (if _light2__on_off_
    (Rendering|Material|SetMaterial _street_light 2 0)
    (else
      (Rendering|Material|SetMaterial _street_light 2 0))))