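; TrackBP is a race track actor for the EasyTrack level that builds its road along a spline.
; The construction script calls PlaceRoad, which loops along the spline in SegmentLength steps, adding a spline mesh component for each segment.
; Segment endpoints use local-space spline locations, with unit directions as tangents.
; Any remainder no longer than one segment stays unfilled, and the event graph does nothing at runtime.
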(event EventBeginPlay)

(event Collision|EventActorBeginOverlap
  (params (OtherActor :type Actor%20Object%20Reference)))

(event EventTick
  (params (DeltaSeconds :type Float%20%28single-precision%29)))

(fn ConstructionScript
  (CallFunction|PlaceRoad))

(fn PlaceRoad
  (bind _spline (Variables|Default|GetSpline))
  (if (> (Spline|GetSplineLength (Variables|Default|GetSpline)) (+ (LocalVariables|GetPlacingDistance) (LocalVariables|GetSegmentLength))) :!label _label
    (bind _returnvalue (AddComponent|AddSplineMeshComponent false))
    (SplineMesh|SetStartandEnd _returnvalue (Spline|GetLocationatDistanceAlongSpline _spline (LocalVariables|GetPlacingDistance) "Local") (Spline|GetDirectionatDistanceAlongSpline _spline (LocalVariables|GetPlacingDistance) "Local") (Spline|GetLocationatDistanceAlongSpline _spline (+ (LocalVariables|GetPlacingDistance) (LocalVariables|GetSegmentLength)) "Local") (Spline|GetDirectionatDistanceAlongSpline _spline (+ (LocalVariables|GetPlacingDistance) (LocalVariables|GetSegmentLength)) "Local") true :!class /Script/Engine.SplineMeshComponent)
    (LocalVariables|SetPlacingDistance (+ (LocalVariables|GetPlacingDistance) (LocalVariables|GetSegmentLength)))
    (goto _label)))