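; BP_Arcade is a luminous arcade sign actor with configurable lightbulb materials.
; Its construction script sets seven lightbulb material slots on the Sign component.
; Each slot takes its material from the shared LightbulbMaterials array through its own index variable, Lightbulb1 to Lightbulb7.
; The file contains no runtime logic, so the look is determined at construction.
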(fn ConstructionScript
  (bind _sign (Variables|Default|GetSign))
  (Utilities|FlowControl|Sequence
    (:then_0
      ;[1 1 1] Choose material for Lightbulbs
      (Rendering|Material|SetMaterial _sign 4 (Utilities|Array|Get(acopy) (Variables|Default|GetLightbulb%20Materials) (Variables|Default|GetLightbulb%20№1))))
    (:then_1
      (Rendering|Material|SetMaterial _sign 3 (Utilities|Array|Get(acopy) (Variables|Default|GetLightbulb%20Materials) (Variables|Default|GetLightbulb%20№2))))
    (:then_2
      (Rendering|Material|SetMaterial _sign 9 (Utilities|Array|Get(acopy) (Variables|Default|GetLightbulb%20Materials) (Variables|Default|GetLightbulb%20№3))))
    (:then_3
      (Rendering|Material|SetMaterial _sign 8 (Utilities|Array|Get(acopy) (Variables|Default|GetLightbulb%20Materials) (Variables|Default|GetLightbulb%20№4))))
    (:then_4
      (Rendering|Material|SetMaterial _sign 7 (Utilities|Array|Get(acopy) (Variables|Default|GetLightbulb%20Materials) (Variables|Default|GetLightbulb%20№5))))
    (:then_5
      (Rendering|Material|SetMaterial _sign 6 (Utilities|Array|Get(acopy) (Variables|Default|GetLightbulb%20Materials) (Variables|Default|GetLightbulb%20№6))))
    (:then_6
      (Rendering|Material|SetMaterial _sign 5 (Utilities|Array|Get(acopy) (Variables|Default|GetLightbulb%20Materials) (Variables|Default|GetLightbulb%20№7))))))